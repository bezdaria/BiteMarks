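; Analog clock actor in the StartMenu folder that rotates second, minute and hour hand meshes to show the system time.
; BeginPlay converts Now() into roll offsets for each hand, adding a minute-based fraction to the hour hand.
; The Time event steps the second hand, advancing the others when its roll nears zero.
; Time is bound to a zero-second, non-looping timer, so nothing here drives repeated ticking.
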(event Custom|Time
  (bind _sm_hande_sec (Variables|Default|GetSM_Hande_Sec))
  (Transformation|AddRelativeRotation _sm_hande_sec (Math|Rotator|MakeRotator -6.0 0.0 0.0) false false)
  (if (Math|Float|NearlyEqual(Float) (.roll (Variables|/Script/Engine.SceneComponent|GetRelativeRotation _sm_hande_sec)) 0.0 1.0)
    (Transformation|AddRelativeRotation (Variables|Default|GetSM_Hande_Min) "0.000000,0.000000,-6.000000" false false)
    (Transformation|AddRelativeRotation (Variables|Default|GetSM_Hande_Hour) "0.000000,0.000000,-0.500000" false false)))

(event EventBeginPlay
  (bind _returnvalue (Math|DateTime|Now))
  (bind _returnvalue_2 (Math|Conversions|ToFloat(Integer) (.minute _returnvalue)))
  (bind _returnvalue_3 (Math|Float|MapRangeClamped _returnvalue_2 0.0 6e+01 0.0 -3.6e+02))
  (bind _returnvalue_4 (/ _returnvalue_3 12.0))
  (Transformation|AddRelativeRotation (Variables|Default|GetSM_Hande_Sec) (Math|Rotator|MakeRotator (Math|Float|MapRangeClamped (Math|Conversions|ToFloat(Integer) (.second _returnvalue)) 0.0 6e+01 0.0 -3.6e+02) 0.0 0.0) false false)
  (Transformation|AddRelativeRotation (Variables|Default|GetSM_Hande_Min) (Math|Rotator|MakeRotator _returnvalue_3 0.0 0.0) false false)
  (Transformation|AddRelativeRotation (Variables|Default|GetSM_Hande_Hour) (Math|Rotator|MakeRotator (Math|Float|SelectFloat (+ (Math|Float|MapRangeClamped (Math|Conversions|ToFloat(Integer) (.hour _returnvalue)) 0.0 12.0 0.0 -3.6e+02) _returnvalue_4) (+ (Math|Float|MapRangeClamped 0.0 0.0 24.0 0.0 -3.6e+02) _returnvalue_4) (>= (.hour _returnvalue) 12)) 0.0 0.0) false false)
  (Utilities|Time|SetTimerbyEvent (delegate Custom|Time) 0.0))

(event Collision|EventActorBeginOverlap
  (params (OtherActor :type Actor%20Object%20Reference)))

(event EventTick
  (params (DeltaSeconds :type Float%20%28single-precision%29)))

(fn ConstructionScript)