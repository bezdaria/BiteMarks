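; Murray is a side-view enemy that patrols back and forth along the X axis and damages actors touching its hit box.
; Each tick, a frame-based step counter moves toward a signed limit, driving movement input; on reaching it, the limit flips sign and the sprite rotates.
; On a BoxHit overlap it applies damage, launches itself along +X and pauses patrol movement for two seconds.
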(event OnComponentBeginOverlap(BoxHit)
  (params (OverlappedComponent :type Primitive%20Component%20Object%20Reference) (OtherActor :type Actor%20Object%20Reference) (OtherComp :type Primitive%20Component%20Object%20Reference) (OtherBodyIndex :type Integer) (bFromSweep :type Boolean) (SweepResult :type Hit%20Result%20Structure%20%28by%20ref%29))
  (Game|Damage|ApplyDamage OtherActor 1e+01 0 0)
  (Character|LaunchCharacter "500.000000,0.000000,0.000000" true false)
  (Variables|Default|SetbIsMovementLock true)
  (Utilities|FlowControl|Delay 2.0)
  (Variables|Default|SetbIsMovementLock false))

(event Custom|Follow
  (if (not (Variables|Default|GetbIsMovementLock))
    (Development|PrintString (Utilities|String|ToString(Float) (Variables|Default|GetS1)))
    (Math|Float|CompareFloat (Variables|Default|GetS1) (Variables|Default|GetS)
      (:>
        (Pawn|Input|AddMovementInput "-1.000000,0.000000,0.000000" 1.0 false)
        (Variables|Default|SetS1 (- (Variables|Default|GetS1) 1.0)))
      (:==
        (if (> (Variables|Default|GetS) 0.0)
          ;[1 1 1] меняем значение на противоположное
          (Variables|Default|SetS (* (Variables|Default|GetS) -1.0))
          (Transformation|SetRelativeRotation (Variables|Default|GetSprite) "0.000000,180.000000,0.000000" false false)
          (else
            (Variables|Default|SetS (* (Variables|Default|GetS) -1.0))
            (Transformation|SetRelativeRotation (Variables|Default|GetSprite) "0.000000,0.000000,0.000000" false false))))
      (:<
        (Pawn|Input|AddMovementInput "1.000000,0.000000,0.000000" 1.0 false)
        (Variables|Default|SetS1 (+ (Variables|Default|GetS1) 1.0))))))

(event EventBeginPlay)

(event Collision|EventActorBeginOverlap
  (params (OtherActor :type Actor%20Object%20Reference)))

(event EventTick
  (params (DeltaSeconds :type Float%20%28single-precision%29))
  (CallFunction|Follow))

(fn ConstructionScript)